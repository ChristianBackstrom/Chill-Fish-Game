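; BP_Menu3D is a 3D menu actor that hosts a Menu3D_Widget and moves the player's view between linked menu actors.
; The widget's TransitionToLinkedMenu event supplies an index into LinkedMenus, and a valid index starts a transition.
; TransitionTo moves collision to the target menu, blends the view target to it with ease-in-out, and disables the player's input on this actor for the blend's duration.
; Collision starts disabled on BeginPlay.
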(event `self.ReceiveBeginPlay`
  (bind _asmenu_3d_widget (cast `/Game/Levels/3DMenu/Widgets/Menu3D_Widget` (`WidgetComponent.GetUserWidgetObject` (`self.Widget`))))
  (add `/Game/Levels/3DMenu/Widgets/Menu3D_Widget.TransitionToLinkedMenu` _asmenu_3d_widget (delegate `OnTransitionBetweenMenus`))
  (`self.SetActorEnableCollision` false))

(event `OnTransitionBetweenMenus`
  (params (MenuIndex :type Integer))
  (if (`KismetArrayLibrary.Array_IsValidIndex` (`self.LinkedMenus`) MenuIndex)
    (`self.TransitionTo` (`|GetArrayItem` (`self.LinkedMenus`) MenuIndex))))

(event `TransitionTo`
  (params (NewMenu :type "/Game/Levels/3DMenu/BP_Menu3D Object Reference"))
  (bind _returnvalue (`GameplayStatics.GetPlayerController` 0))
  (bind _blend_time (`self.Blend Time`))
  (`self.SetActorEnableCollision` false)
  (`self.SetActorEnableCollision` NewMenu true)
  (`PlayerController.SetViewTargetWithBlend` _returnvalue NewMenu _blend_time "VTBlend_EaseInOut" 2.0 true)
  (`self.DisableInput` _returnvalue)
  (`KismetSystemLibrary.Delay` _blend_time)
  (`self.EnableInput` _returnvalue))

(fn `UserConstructionScript`)