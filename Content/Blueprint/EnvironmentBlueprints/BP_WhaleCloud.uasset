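; BP_WhaleCloud is an environment actor that travels along the spline of a referenced actor, starting at BeginPlay.
; A timeline with its play rate set to the inverse of TimeToComplete drives an alpha that is scaled to distance along the spline.
; Each update sets the actor's transform from that distance, taking location in world space but rotation in the spline's local space.
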(event `self.ReceiveBeginPlay`
  (`self.MoveObj`))

(event `MoveObj`
  (bind _spline (`/Game/Blueprint/EnvironmentBlueprints/CloudSpline.Spline` (`self.SplineRef`)))
  (`TimelineComponent.SetPlayRate` (`self.MoveObjTimeline`) (/ 1.0 (`self.TimeToComplete`)))
  (bind (_direction _movetrack) (`Timeline|MoveObjTimeline`)
    (:`Update`
      (bind _returnvalue (`KismetMathLibrary.Lerp` 0.0 (`SplineComponent.GetSplineLength` (`/Game/Blueprint/EnvironmentBlueprints/CloudSpline.Spline` (`self.SplineRef`))) _movetrack))
      (`self.K2_SetActorTransform` (`KismetMathLibrary.MakeTransform` (`SplineComponent.GetLocationAtDistanceAlongSpline` _spline _returnvalue "World") (`SplineComponent.GetRotationAtDistanceAlongSpline` _spline _returnvalue "Local"))))))

(fn `UserConstructionScript`)