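; Aurora borealis actor that moves back and forth along a referenced spline, starting at BeginPlay.
; A timeline, with play rate scaled by TimeToComplete, lerps distance along the spline to set world location and rotation, with a 90-degree pitch offset.
; When the timeline finishes, it reverses, waits TimeToComplete, then plays again to keep the motion cycling.
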(event `self.ReceiveBeginPlay`
  (`self.MoveObj`))

(event `Play`
  (bind _spline (`/Game/Blueprint/EnvironmentBlueprints/AuroraSpline.Spline` (`self.SplineRef`)))
  (bind (_direction _movetrack) (`Timeline|Timeline` :!label _label)
    (:`Update`
      (bind _returnvalue (`KismetMathLibrary.Lerp` 0.0 (`SplineComponent.GetSplineLength` (`/Game/Blueprint/EnvironmentBlueprints/AuroraSpline.Spline` (`self.SplineRef`))) _movetrack))
      (`self.K2_SetActorLocationAndRotation` (`SplineComponent.GetLocationAtDistanceAlongSpline` _spline _returnvalue "World") (`KismetMathLibrary.ComposeRotators` (`SplineComponent.GetRotationAtDistanceAlongSpline` _spline _returnvalue "World") (struct :`Roll` 90.0))))
    (:`Finished`
      (`self.Reverse`)
      (`KismetSystemLibrary.Delay` (`self.TimeToComplete`))
      (`self.Play`))))

(event `MoveObj`
  (`TimelineComponent.SetPlayRate` (`self.Timeline`) (/ 1.0 (`self.TimeToComplete`)))
  (goto _label :!via `PlayFromStart`))

(event `Reverse`
  (goto _label :!via `Reverse`))

(fn `UserConstructionScript`)