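; Small upgrade pickup that applies a random bubble stat boost when the bubble actor overlaps its sphere; it is not destroyed afterwards.
; GetRandomUpgrade rerolls at each nested check, so odds are uneven and sometimes nothing is applied.
; Upgrades raise lifetime, speed, max size or charge time, or lower minimum charge time.
; Each updates every Bubble_ShooterInterface actor through interface getters and setters, with debug prints throughout.
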(event `self.Sphere.OnComponentBeginOverlap`
  (params (OverlappedComponent :type "PrimitiveComponent Object Reference") (OtherActor :type "Actor Object Reference") (OtherComp :type "PrimitiveComponent Object Reference") (OtherBodyIndex :type Integer) (bFromSweep :type Boolean) (SweepResult :type "HitResult Structure (by ref)"))
  (`KismetSystemLibrary.PrintString` "collided")
  (bind _bubbleactor (message `/Game/Blueprint/Weapon/Bubble_Interface.GetBubbleActor` OtherActor))
  (if (== _bubbleactor OtherActor)
    (`KismetSystemLibrary.PrintString` "collided with bubble")
    (`self.GetRandomUpgrade`)))

(fn `ChargeTimeUpgrade`
  (`KismetSystemLibrary.PrintString` "ChargeTimeUpgrade")
  (bind _outactors (`GameplayStatics.GetAllActorsWithInterface` "/Game/Blueprint/Weapon/Bubble_ShooterInterface.Bubble_ShooterInterface_C"))
  (for _array_element _outactors
    (bind _bubblechargetime (message `/Game/Blueprint/Weapon/Bubble_ShooterInterface.GetBubbleChargeTime` _array_element))
    (bind _result (`/Engine/EditorBlueprintResources/StandardMacros.IncrementFloat` _bubblechargetime)
      (:`  `
        (message `/Game/Blueprint/Weapon/Bubble_ShooterInterface.SetBubbleChargeTime` _array_element _result)
        (`KismetSystemLibrary.PrintString` "BubbleUpgraded!")))))

(fn `GetRandomUpgrade`
  (bind _returnvalue (`KismetMathLibrary.RandomIntegerInRange` 1 5))
  (`KismetSystemLibrary.PrintString` "choosing random upgrade")
  (if (== _returnvalue 1)
    (`self.LifeTimeUpgrade`)
    (elif (== _returnvalue 2)
      (`self.SpeedUpgrade`)
      (elif (== _returnvalue 3)
        (`self.SizeUpgrade`)
        (elif (== _returnvalue 4)
          (`self.MinChargeTimeUpgrade`)
          (elif (== _returnvalue 5)
            (`self.ChargeTimeUpgrade`)))))))

(fn `LifeTimeUpgrade`
  (`KismetSystemLibrary.PrintString` "LifeTimeUpgrade")
  (bind _outactors (`GameplayStatics.GetAllActorsWithInterface` "/Game/Blueprint/Weapon/Bubble_ShooterInterface.Bubble_ShooterInterface_C"))
  (for _array_element _outactors
    (bind _lifetime (message `/Game/Blueprint/Weapon/Bubble_ShooterInterface.GetBubbleLifeTime` _array_element))
    (bind _result (`/Engine/EditorBlueprintResources/StandardMacros.IncrementFloat` _lifetime)
      (:`  `
        (message `/Game/Blueprint/Weapon/Bubble_ShooterInterface.SetBubbleLifeTime` _array_element _result)
        (`KismetSystemLibrary.PrintString` "BubbleUpgraded!")))))

(fn `MinChargeTimeUpgrade`
  (`KismetSystemLibrary.PrintString` "MinChargeTimeUpgrade")
  (bind _outactors (`GameplayStatics.GetAllActorsWithInterface` "/Game/Blueprint/Weapon/Bubble_ShooterInterface.Bubble_ShooterInterface_C"))
  (for _array_element _outactors
    (bind _minchargetime (message `/Game/Blueprint/Weapon/Bubble_ShooterInterface.GetBubbleMinChargeTime` _array_element))
    (message `/Game/Blueprint/Weapon/Bubble_ShooterInterface.SetBubbleMinChargeTime` _array_element (- _minchargetime 0.05))
    (`KismetSystemLibrary.PrintString` "BubbleUpgraded!")))

(fn `SizeUpgrade`
  (`KismetSystemLibrary.PrintString` "SizeUpgrade")
  (bind _outactors (`GameplayStatics.GetAllActorsWithInterface` "/Game/Blueprint/Weapon/Bubble_ShooterInterface.Bubble_ShooterInterface_C"))
  (for _array_element _outactors
    (bind _bubblemaxsize (message `/Game/Blueprint/Weapon/Bubble_ShooterInterface.GetBubbleMaxSize` _array_element))
    (bind _result (`/Engine/EditorBlueprintResources/StandardMacros.IncrementFloat` _bubblemaxsize)
      (:`  `
        (message `/Game/Blueprint/Weapon/Bubble_ShooterInterface.SetBubbleMaxSize` _array_element _result)
        (`KismetSystemLibrary.PrintString` "BubbleUpgraded!")))))

(fn `SpeedUpgrade`
  (`KismetSystemLibrary.PrintString` "SpeedUpgrade")
  (bind _outactors (`GameplayStatics.GetAllActorsWithInterface` "/Game/Blueprint/Weapon/Bubble_ShooterInterface.Bubble_ShooterInterface_C"))
  (for _array_element _outactors
    (bind _bubblespeed (message `/Game/Blueprint/Weapon/Bubble_ShooterInterface.GetBubbleSpeed` _array_element))
    (bind _result (`/Engine/EditorBlueprintResources/StandardMacros.IncrementFloat` _bubblespeed)
      (:`  `
        (message `/Game/Blueprint/Weapon/Bubble_ShooterInterface.SetBubbleSpeed` _array_element _result)
        (`KismetSystemLibrary.PrintString` "BubbleUpgraded!")))))

(fn `UserConstructionScript`)