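; BP_Objective is a score-gated checkpoint that holds BP_MovingBoat until the player reaches a required fishing score.
; BeginPlay gets the score reference through a message call on the game mode.
; Box overlap stores the boat, then either destroys the objective if the score suffices or stops the boat and sets its objective.
; Tick polls the score, then clears the objective, restarts the stored boat and destroys the actor.
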(event `self.ReceiveBeginPlay`
  ;[1 0.8459 0.44] Getting score reference
  (bind _gamemode (message `/Game/Blueprint/BP_GameMode_Interface.GetFishingGameMode` (`GameplayStatics.GetGameMode`)))
  (set `self.ScoreRef` _gamemode))

(event `self.Box.OnComponentBeginOverlap`
  (params (OverlappedComponent :type "PrimitiveComponent Object Reference") (OtherActor :type "Actor Object Reference") (OtherComp :type "PrimitiveComponent Object Reference") (OtherBodyIndex :type Integer) (bFromSweep :type Boolean) (SweepResult :type "HitResult Structure (by ref)"))
  ;[0.8649 0.7498 1] Stopping boat to complete objective
  (bind _asbp_moving_boat (cast `/Game/Blueprint/BoatMechanics/BP_MovingBoat` OtherActor))
  (bind _output_get (set `self.BoatRef` _asbp_moving_boat))
  (if (>= (`/Game/Blueprint/BP_FishingGamemode.Score` (`self.ScoreRef`)) (`self.ScoreNeeded`))
    (`self.K2_DestroyActor`)
    (else
      (`|ExecutionSequence`
        (:`then_0`
          (`/Game/Blueprint/BoatMechanics/BP_MovingBoat.Stop Boat` _output_get))
        (:`then_1`
          (set `/Game/Blueprint/BoatMechanics/BP_MovingBoat.CurrentObjective` (`self.Objective`) _output_get))))))

(event `self.ReceiveTick`
  (params (DeltaSeconds :type "Float (single-precision)"))
  ;[1 0.5849 0.7061] Starting the boat after objective is met
  (if (>= (`/Game/Blueprint/BP_FishingGamemode.Score` (`self.ScoreRef`)) (`self.ScoreNeeded`))
    (set `/Game/Blueprint/BoatMechanics/BP_MovingBoat.CurrentObjective` "" (`self.BoatRef`))
    (`/Game/Blueprint/BoatMechanics/BP_MovingBoat.Start Boat` (`self.BoatRef`))
    (`self.K2_DestroyActor`)))

(fn `UserConstructionScript`)