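; BP_BubbleUpgradeHandler runs the upgrade choice screen shown when an objective is completed, letting the player pick a bubble.
; It creates the unlock widget at BeginPlay, then on completion shows it with UI-only input and a cursor, adding one button per bubble class using its default image.
; A click passes the bubble at that button's index to ChoosenBubble, removes the widget, restores game input and clears the list.
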(event `self.ReceiveBeginPlay`
  (bind _returnvalue (`|CreateWidget` "/Game/UI/WBP_UpgradedBubbleUnlockUI.WBP_UpgradedBubbleUnlockUI_C" (`GameplayStatics.GetPlayerController` 0)))
  (set `self.UI` _returnvalue))

(event `self.ObjectiveCompleted`
  (params (Bubbles :type "Array of Bubble Class Reference (by ref)"))
  (`WidgetBlueprintLibrary.SetInputMode_UIOnlyEx` (`GameplayStatics.GetPlayerController` 0) (`self.UI`) "LockOnCapture")
  (set `self.Bubbles` Bubbles)
  (`UserWidget.AddToViewport` (`self.UI`) 0)
  (set `PlayerController.bShowMouseCursor` true (`GameplayStatics.GetPlayerController` 0))
  (for (_array_element _array_index) Bubbles
    (bind _newparam (`/Game/UI/WBP_UpgradedBubbleUnlockUI.Addbutton` (`self.UI`) (defaults `Object` _array_element)))
    (set `/Game/UI/WBP_ImageButton.Index` _array_index _newparam)
    (add `/Game/UI/WBP_ImageButton.OnClicked` _newparam (delegate `Selected`))))

(event `Selected`
  (params (Index :type Integer))
  (bind _returnvalue (`GameplayStatics.GetPlayerController` 0))
  (`self.ChoosenBubble` (`|GetArrayItem` (`self.Bubbles`) Index))
  (`Widget.RemoveFromParent` (`self.UI`))
  (`WidgetBlueprintLibrary.SetInputMode_GameOnly` _returnvalue)
  (set `PlayerController.bShowMouseCursor` false _returnvalue)
  (`KismetArrayLibrary.Array_Clear` (`self.Bubbles`)))

(fn `UserConstructionScript`)