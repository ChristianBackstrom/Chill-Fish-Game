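; BP_NarrativeManager presents dialogue, handling both the on-screen text window and the audio for each line.
; Dialogue events add or remove a WBP_DialogueWindow and push text to it, with the end event also firing and then clearing DialogueEnded bindings.
; Each new line with a valid sound plays through one reused audio component, created on demand attached to BP_Fishmount, and stops when the line ends.
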(event `self.ReceiveBeginPlay`
  ;[1 1 1] Creating UI
  (`self.Create Widget`)
  (`self.Create Audio Comp`))

(event `self.DialogueStarted`
  ;[1 1 1] Adding And Removing from viewport
  (`/Engine/EditorBlueprintResources/StandardMacros.IsValid` (`self.Dialogue UI`)
    (:`Is Valid`
      _)
    (:`Is Not Valid`
      (`self.Create Widget`)))
  (`UserWidget.AddToViewport` (`self.Dialogue UI`) 0))

(event `self.EndDialogue`
  ;[1 1 1] Adding And Removing from viewport
  (`Widget.RemoveFromParent` (`self.Dialogue UI`))
  (`self.DialogueEnded`)
  (clear `self.DialogueEnded`))

(event `self.TextUpdated`
  (params (Text :type String))
  ;[1 1 1] Updating Text
  (`/Game/UI/Dialogue/WBP_DialogueWindow.Set Text` (`self.Dialogue UI`) Text))

(event `self.StartedNextLine`
  ;[1 1 1] Sound
  (`/Engine/EditorBlueprintResources/StandardMacros.IsValid` (`self.CurrentSound`)
    (:`Is Valid`
      (`self.Create Audio Comp`)
      (if (`AudioComponent.IsPlaying` (`self.AudioComp`))
        (`AudioComponent.Stop` (`self.AudioComp`)))
      (`AudioComponent.SetSound` (`self.AudioComp`) (`self.CurrentSound`))
      (`AudioComponent.Play` (`self.AudioComp`) 0.0))))

(event `self.EndLine`
  ;[1 1 1] Sound
  (`AudioComponent.Stop` (`self.AudioComp`)))

(fn `Create Audio Comp`
  (`/Engine/EditorBlueprintResources/StandardMacros.IsValid` (`self.AudioComp`)
    (:`Is Not Valid`
      (bind _returnvalue (`GameplayStatics.GetActorOfClass` "/Game/Art/StaticMeshes/BP_Fishmount.BP_Fishmount_C"))
      (`/Engine/EditorBlueprintResources/StandardMacros.IsValid` _returnvalue
        (:`Is Valid`
          (bind _returnvalue_2 (`GameplayStatics.SpawnSoundAttached` "/Game/Music/152.152" (`/Game/Art/StaticMeshes/BP_Fishmount.DefaultSceneRoot` _returnvalue) "None" (0.0 0.0 0.0) (struct) "KeepRelativeOffset" false 1.0 1.0 0.0 "/Game/SFX/SA_BasicSoundAttenuation.SA_BasicSoundAttenuation" null false))
          (set `self.AudioComp` _returnvalue_2))))))

(fn `Create Widget`
  (`/Engine/EditorBlueprintResources/StandardMacros.IsValid` (`self.Dialogue UI`)
    (:`Is Not Valid`
      (bind _returnvalue (`|CreateWidget` "/Game/UI/Dialogue/WBP_DialogueWindow.WBP_DialogueWindow_C" (`GameplayStatics.GetPlayerController` 0)))
      (set `self.Dialogue UI` _returnvalue))))

(fn `UserConstructionScript`)