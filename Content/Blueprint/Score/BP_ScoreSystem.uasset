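; BP_ScoreSystem tracks the score for a fishing game.
; FishesCaught sums each fish's value times its size, then applies a growing combo multiplier while accumulated time since combo start stays within ComboTime.
; A bonus for multiple fish in one catch scales the total, which is rounded and passed to AddScore.
; RemoveScore sets Score to the given amount minus the current Score, reversing the usual subtraction order.
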(event `self.ReceiveBeginPlay`)

(fn `AddScore`
  (params (AmountToAdd :type Integer))
  (set `self.Score` (+ (`self.Score`) AmountToAdd)))

(fn `FishesCaught`
  (params (`Fish Value` :type "Array of Integer") (`Fish Size` :type "Array of Float (double-precision)"))
  (locals (ScoreCounter :type "Float (double-precision)"))
  (set `local.ScoreCounter` 0.0)
  ;[1 1 1] Adding together all fish in catch
  (for (_array_element _array_index) `Fish Value`
    (set `local.ScoreCounter` (+ (* _array_element (`|GetArrayItem` `Fish Size` _array_index)) (`local.ScoreCounter`))))
  ;[1 1 1] Combo multiplier logic
  (if (> (`self.LastTimeCaught`) 0.0)
    (bind _output_get (set `self.TimeSinceComboStart` (+ (`self.TimeSinceComboStart`) (- (`GameplayStatics.GetTimeSeconds`) (`self.LastTimeCaught`)))))
    (if (> _output_get (`self.ComboTime`))
      (set `self.FishCaughtDuringCombo` 0)
      (set `self.TimeSinceComboStart` 0.0)
      (else
        (set `local.ScoreCounter` (* (`local.ScoreCounter`) (+ (`self.BaseComboMultiplier`) (* (`self.FishCaughtDuringCombo`) (`self.ComboMultiplierIncreaseValue`)))))
        (set `self.FishCaughtDuringCombo` (+ (`self.FishCaughtDuringCombo`) 1)))))
  (set `self.LastTimeCaught` (`GameplayStatics.GetTimeSeconds`))
  (`self.AddScore` (`KismetMathLibrary.Round` (* (`local.ScoreCounter`) (+ (* (- (`KismetArrayLibrary.Array_Length` `Fish Value`) 1) (`self.BonusForMultipleFish%`)) 1.0)))))

(fn `RemoveScore`
  (params (AmountToRemove :type Integer))
  (set `self.Score` (- AmountToRemove (`self.Score`))))

(fn `UserConstructionScript`)