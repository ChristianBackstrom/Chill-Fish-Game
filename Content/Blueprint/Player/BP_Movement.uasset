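; BP_Movement is a player Blueprint handling the aim widget, footstep audio, fish name display and pausing.
; Each Tick, it plays random timed footstep sounds while moving and line-traces from the camera to show the looked-at fish's widget, hiding the previous one.
; Enhanced Input actions toggle a lazily created pause menu with matching cursor and input mode, and trigger a narrator honk sound on a combo.
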(event `self.ReceiveBeginPlay`
  (bind _returnvalue (`|CreateWidget` "/Game/UI/WBP_Aim.WBP_Aim_C" (`GameplayStatics.GetPlayerController` 0)))
  (`UserWidget.AddToViewport` _returnvalue 0))

(event `self.ReceiveTick`
  (params (DeltaSeconds :type "Float (single-precision)"))
  (bind _returnvalue (`GameplayStatics.GetPlayerCameraManager` 0))
  (bind _fish (`self.Fish`))
  (bind _fish_2 (`self.Fish`))
  (bind _returnvalue_2 (`self.K2_GetActorLocation` _returnvalue))
  ;[1 1 1] Fish name widget
  ;[1 1 1] Footstep logic
  (`self.Footsteps`)
  (bind (_outhit _returnvalue_3) (`KismetSystemLibrary.LineTraceSingleForObjects` _returnvalue_2 (+ _returnvalue_2 (* (`self.GetActorForwardVector` _returnvalue) (`self.Range`))) (`|MakeArray` (enumliteral `EObjectTypeQuery` "ObjectTypeQuery7"))))
  (if _returnvalue_3
    (bind _asbp_fish_actor (cast `/Game/Blueprint/Fish/BP_FishActor` (`.HitActor` (`GameplayStatics.BreakHitResult` _outhit))))
    (if (== _asbp_fish_actor (`self.Fish`))
      (`SceneComponent.SetHiddenInGame` (`/Game/Blueprint/Fish/BP_FishActor.Widget` _asbp_fish_actor) false false)
      (else
        (`/Engine/EditorBlueprintResources/StandardMacros.IsValid` _fish
          (:`Is Valid`
            (`SceneComponent.SetHiddenInGame` (`/Game/Blueprint/Fish/BP_FishActor.Widget` _fish) true false))
          (:`Is Not Valid`
            _))
        (set `self.Fish` _asbp_fish_actor)))
    (else
      (`/Engine/EditorBlueprintResources/StandardMacros.IsValid` _fish_2
        (:`Is Valid`
          (`SceneComponent.SetHiddenInGame` (`/Game/Blueprint/Fish/BP_FishActor.Widget` _fish_2) true false))))))

(event `EnhancedInput|/Game/Input/InputActions/IA_Pause`
  (params (ActionValue :type Boolean) (ElapsedSeconds :type "Float (double-precision)") (TriggeredSeconds :type "Float (double-precision)") (InputAction :type "InputAction Object Reference" :default "/Game/Input/InputActions/IA_Pause.IA_Pause"))
  (bind _returnvalue (`GameplayStatics.GetPlayerController` 0))
  (bind _pause_menu_ref (`self.Pause Menu REF`))
  ;[1 1 1] Pause/Unpause Game
  (:`Started`
    (`/Engine/EditorBlueprintResources/StandardMacros.IsValid` (`self.Pause Menu REF`)
      (:`Is Valid`
        _)
      (:`Is Not Valid`
        (bind _returnvalue_2 (`|CreateWidget` "/Game/Levels/PauseMenu/PauseMenuWidget.PauseMenuWidget_C"))
        (set `self.Pause Menu REF` _returnvalue_2)))
    (if (`GameplayStatics.IsGamePaused`)
      (`Widget.RemoveFromParent` _pause_menu_ref)
      (`GameplayStatics.SetGamePaused` false)
      (set `PlayerController.bShowMouseCursor` false _returnvalue)
      (`WidgetBlueprintLibrary.SetInputMode_GameOnly` _returnvalue)
      (else
        (`UserWidget.AddToViewport` _pause_menu_ref 0)
        (`GameplayStatics.SetGamePaused` true)
        (set `PlayerController.bShowMouseCursor` true _returnvalue)
        (`WidgetBlueprintLibrary.SetInputMode_GameAndUIEx` _returnvalue _pause_menu_ref "LockInFullscreen" false)))))

(event `EnhancedInput|/Game/Input/InputActions/Combo/IA_Combo`
  (params (ActionValue :type Boolean) (ElapsedSeconds :type "Float (double-precision)") (TriggeredSeconds :type "Float (double-precision)") (InputAction :type "InputAction Object Reference" :default "/Game/Input/InputActions/Combo/IA_Combo.IA_Combo"))
  (:`Triggered`
    (`GameplayStatics.PlaySoundAtLocation` "/Game/SFX/HonkHonk/Narrator_Honk_02.Narrator_Honk_02" (`self.K2_GetActorLocation`) (struct) 1.0 1.0 0.0 null null null null)))

(fn `Footsteps`
  (locals (Footsteps :type "Array of SoundBase Object Reference"))
  (bind _footsteps (`local.Footsteps`))
  ;[1 1 1] If moving
  (if (> (`KismetMathLibrary.VSize` (`self.GetVelocity`)) 0.0)
    (set `self.IsMoving` true)
    (if (> (- (`GameplayStatics.GetTimeSeconds`) (`self.LastFootStepTime`)) (`self.TimeBetweenFootsteps`))
      (set `self.LastFootStepTime` (`GameplayStatics.GetTimeSeconds`))
      (`GameplayStatics.PlaySound2D` (`|GetArrayItem` _footsteps (`KismetMathLibrary.RandomIntegerInRange` 0 (- (`KismetArrayLibrary.Array_Length` _footsteps) 1))) 0.3 1.0 0.0 null null))
    (else
      (set `self.IsMoving` false))))

(fn `UserConstructionScript`)