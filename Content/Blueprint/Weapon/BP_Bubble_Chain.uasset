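; Bubble weapon actor that chains one fish catch to other nearby fish.
; FishCaught builds a list of up to MaxFish extra targets by repeatedly sphere-tracing for the closest unlisted fish within Range of the last pick.
; A custom ForEachLoopSequence macro then steps through them one at a time, waiting on the BubbleMovement timeline.
; Each step flies a spawned BP_Bubble to its fish, forces the overlap catch and starts the next hop there.
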(event `self.FishCaught`
  (params (FishActor :type "FishActor Object Reference"))
  (bind _returnvalue (`self.K2_GetActorLocation`))
  (bind _foundactors (`self.FoundActors`))
  (bind _nearestactor (`self.NearestActor`))
  (bind _newlocation (`self.NewLocation`))
  (bind _returnvalue_2 (`KismetArrayLibrary.Array_Length` _foundactors))
  (`KismetArrayLibrary.Array_AddUnique` _foundactors FishActor)
  (set `self.NewLocation` _returnvalue)
  (for _ (range 1 (+ (`self.MaxFish`) 1))
    (bind _outhits (`KismetSystemLibrary.SphereTraceMulti` _newlocation _newlocation (`self.Range`) "TraceTypeQuery1" false _foundactors))
    (for _array_element _outhits
      (bind (_bblockinghit _binitialoverlap _time _distance _location _impactpoint _normal _impactnormal _physmat _hitactor) (`GameplayStatics.BreakHitResult` _array_element))
      ;[1 1 1] Check for Closest Fish
      (if (< _distance (`self.NearestActorDistance`))
        (if (`GameplayStatics.ObjectIsA` _hitactor "/Script/GP3Team04.FishActor")
          (`|ExecutionSequence`
            (:`then_0`
              (set `self.NearestActorDistance` _distance))
            (:`then_1`
              (set `self.NearestActor` _hitactor))))))
    ;[1 1 1] Generate which fishes should be caught
    (set `self.NearestActorDistance` 10000.0)
    (`/Engine/EditorBlueprintResources/StandardMacros.IsValid` _nearestactor
      (:`Is Valid`
        (`KismetArrayLibrary.Array_AddUnique` (`self.FoundActors`) _nearestactor)
        (set `self.NewLocation` (`self.K2_GetActorLocation` _nearestactor)))))
  (if (> _returnvalue_2 1)
    (set `self.NewLocation` _returnvalue)
    (bind (_array_element_2 _array_index) (`self.ForEachLoopSequence` _foundactors 1 :!label _label)
      (:`Loop Body`
        (`KismetSystemLibrary.PrintString` (`KismetStringLibrary.Conv_IntToString` _array_index) true true (struct :`R` 1.0 :`G` 0.045439 :`A` 1.0) 5.0)
        (bind _output_get (set `self.NearestActor` _array_element_2))
        (bind _returnvalue_3 (`|SpawnActorFromClass` "/Game/Blueprint/Weapon/BP_Bubble.BP_Bubble_C" (`KismetMathLibrary.Conv_VectorToTransform` (`self.NewLocation`)) "Undefined" "OverrideRootScale" null null))
        (`KismetSystemLibrary.PrintString` "Spawned Bubble" true true (struct :`R` 1.0 :`G` 0.045439 :`A` 1.0) 5.0)
        (`TimelineComponent.SetPlayRate` (`self.BubbleMovement`) (* (+ (`self.FloatDuration`) 0.1) (- _returnvalue_2 0.0)))
        (bind (_direction _bubbletrack) (`Timeline|BubbleMovement` :!via `PlayFromStart`)
          (:`Update`
            (bind _returnvalue_4 (`self.K2_GetActorLocation` _output_get))
            (`self.K2_SetActorLocation` _returnvalue_3 (`KismetMathLibrary.VLerp` (`self.K2_GetActorLocation` _returnvalue_3) _returnvalue_4 _bubbletrack) false false))
          (:`Finished`
            (set `self.NewLocation` _returnvalue_4)
            (set `Bubble.bShouldCoolide` true _returnvalue_3)
            (set `Bubble.bIgnoreSize` true _returnvalue_3)
            (`self.OnOverlapBegin` _returnvalue_3 null (`self.NearestActor`) null 0 false (`self.Sweep Result`))
            (`KismetSystemLibrary.PrintString` "Catched Fish" true true (struct :`R` 0.032125 :`G` 1.0 :`A` 1.0) 5.0)
            (goto _label :!via `Next`))))
      (:`Completed`
        (`KismetArrayLibrary.Array_Clear` _foundactors :!label _label_2)
        (`KismetSystemLibrary.PrintString` "LoopDone" true true (struct :`R` 0.143823 :`G` 1.0 :`A` 1.0) 5.0)))
    (else
      (goto _label_2))))

(fn `UserConstructionScript`
  (`parent.UserConstructionScript`))