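; Bubble-shooting wand weapon that creates an upgraded-bubble cooldown UI and exposes bubble stats through interface events and getters.
; BeginPlay positions the Wand and fills the widget from UpgradedBubbles; Tick pushes cooldowns and timers to it, and ChangedBubble highlights the selected bubble.
; Fired plays the shot sound, while StartAim and StopAim ease the Wand between aim and offhand positions.
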(event `self.ChangedBubble`
  (params (Index :type Integer))
  (for (_array_element _array_index) (`/Game/UI/WBP_UpgradedBubbleUI.Bubbles` (`self.Cooldown`))
    (`/Game/UI/WBP_BubbleSlots.IsSelected` _array_element (== _array_index Index))))

(event `self.ReceiveTick`
  (params (DeltaSeconds :type "Float (single-precision)"))
  (`/Game/UI/WBP_UpgradedBubbleUI.UpdatedCooldown` (`self.Cooldown`) (`self.Cooldowns`) (`self.Timers`)))

(event `self.ReceiveBeginPlay`
  (`SceneComponent.K2_SetRelativeLocation` (`self.Wand`) (30.0 0.0 -10.0) false false)
  (bind _returnvalue (`|CreateWidget` "/Game/UI/WBP_UpgradedBubbleUI.WBP_UpgradedBubbleUI_C" (`GameplayStatics.GetPlayerController` 0)))
  (bind _output_get (set `self.Cooldown` _returnvalue))
  (`UserWidget.AddToViewport` _output_get 0)
  (`/Game/UI/WBP_UpgradedBubbleUI.InstantiateBubbles` _output_get (`self.UpgradedBubbles`)))

(event `self.Fired`
  (`AudioComponent.Play` (`self.MS_BubbleShotSound`) 0.0))

(event `self.StartAim`
  (params (ActionValue :type "InputActionValue Structure (by ref)"))
  (`KismetSystemLibrary.MoveComponentTo` (`self.Wand`) (`self.ADLocation`) (struct) true true))

(event `self.StopAim`
  (params (ActionValue :type "InputActionValue Structure (by ref)"))
  (`KismetSystemLibrary.MoveComponentTo` (`self.Wand`) (`self.OffhandLocation`) (struct) true true))

(event `/Game/Blueprint/Weapon/Bubble_ShooterInterface.SetBubbleMinChargeTime`
  (params (MinChargeTime :type "Float (double-precision)"))
  ;[1 1 1] Interface Events
  (set `self.MinChargeTime` MinChargeTime))

(event `/Game/Blueprint/Weapon/Bubble_ShooterInterface.SetBubbleChargeTime`
  (params (BubbleChargeTime :type "Float (double-precision)"))
  ;[1 1 1] Interface Events
  (set `self.ChargeTime` BubbleChargeTime))

(event `/Game/Blueprint/Weapon/Bubble_ShooterInterface.SetBubbleMaxSize`
  (params (BubbleMaxSize :type "Float (double-precision)"))
  ;[1 1 1] Interface Events
  (set `self.MaxSizeBubble` BubbleMaxSize))

(event `/Game/Blueprint/Weapon/Bubble_ShooterInterface.SetBubbleSpeed`
  (params (BubbleSpeed :type "Float (double-precision)"))
  ;[1 1 1] Interface Events
  (set `self.BubbleBaseSpeed` BubbleSpeed))

(event `/Game/Blueprint/Weapon/Bubble_ShooterInterface.SetBubbleLifeTime`
  (params (LifeTime :type "Float (double-precision)"))
  ;[1 1 1] Interface Events
  (set `self.LifeTime` LifeTime))

(fn `GetBubbleChargeTime`
  (returns (BubbleChargeTime :type "Float (double-precision)"))
  (return (`self.ChargeTime`)))

(fn `GetBubbleLifeTime`
  (returns (LifeTime :type "Float (double-precision)"))
  (return (`self.LifeTime`)))

(fn `GetBubbleMaxSize`
  (returns (BubbleMaxSize :type "Float (double-precision)"))
  (return (`self.MaxSizeBubble`)))

(fn `GetBubbleMinChargeTime`
  (returns (MinChargeTime :type "Float (double-precision)"))
  (return (`self.MinChargeTime`)))

(fn `GetBubbleSHooter`
  (returns (BubbleShooter :type "/Game/Blueprint/Weapon/BP_BubbleShooter Object Reference"))
  (return self))

(fn `GetBubbleSpeed`
  (returns (BubbleSpeed :type "Float (double-precision)"))
  (return (`self.BubbleBaseSpeed`)))

(fn `UserConstructionScript`)