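; A bubble weapon actor that slows fish when popped.
; Its POP event passes TimeDilation to SlowFish through the game mode's message getter, then spawns a pop sound and Niagara effect at the bubble's location.
; GetBubbleActor and GetSlowTimeBubble both return the actor itself.
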(event `self.POP`
  (bind _returnvalue (`self.K2_GetActorLocation`))
  (`|ExecutionSequence`
    (:`then_0`
      (bind _gamemode (message `/Game/Blueprint/BP_GameMode_Interface.GetFishingGameMode` (`GameplayStatics.GetGameMode`)))
      (`/Game/Blueprint/BP_FishingGamemode.SlowFish` _gamemode (`self.TimeDilation`)))
    (:`then_1`
      (`GameplayStatics.SpawnSoundAtLocation` "/Game/SFX/MS_BubblePopSound.MS_BubblePopSound" _returnvalue (struct) 1.0 1.0 0.0 null null))
    (:`then_2`
      (`NiagaraFunctionLibrary.SpawnSystemAtLocation` "/Game/VFX/NG_BubblePop.NG_BubblePop" _returnvalue))))

(fn `GetBubbleActor`
  (returns (BubbleActor :type "Bubble Object Reference"))
  (return self))

(fn `GetSlowTimeBubble`
  (returns (`BP SLowTimeBubble` :type "/Game/Blueprint/Weapon/BP_Bubble_TimeSlow Object Reference"))
  (return self))

(fn `UserConstructionScript`
  (`parent.UserConstructionScript`))