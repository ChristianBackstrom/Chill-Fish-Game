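; Exploding bubble weapon actor that bursts into smaller BP_Bubble actors when its POP event fires.
; POP spawns bubbles at its location with random rotation and scale, skipping blocked spawns, and collects them in an array.
; It then enables movement and collision and sets speed on each through GetBubbleActorMessage.
; The lifespan call in that loop targets the last spawn result rather than the current array element.
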(event `self.POP`
  (bind _returnvalue (`KismetMathLibrary.RandomFloatInRange` 1.0 1.5))
  (bind _arrayofbubble (`self.ArrayOfBubble`))
  (for _ (range (+ (`self.AmountOfBubblesExploding`) 1))
    (bind _returnvalue_2 (`|SpawnActorFromClass` "/Game/Blueprint/Weapon/BP_Bubble.BP_Bubble_C" (`KismetMathLibrary.MakeTransform` (`self.K2_GetActorLocation` self) (`KismetMathLibrary.MakeRotator` (`KismetMathLibrary.RandomFloatInRange` 0.0 360.0) (`KismetMathLibrary.RandomFloatInRange` 0.0 360.0) (`KismetMathLibrary.RandomFloatInRange` 0.0 360.0)) (`KismetMathLibrary.MakeVector` _returnvalue _returnvalue _returnvalue)) "AdjustIfPossibleButDontSpawnIfColliding" "OverrideRootScale" null null))
    (`KismetArrayLibrary.Array_Add` _arrayofbubble _returnvalue_2))
  (for _array_element _arrayofbubble
    (bind _bubbleactor (message `/Game/Blueprint/Weapon/Bubble_Interface.GetBubbleActor` _array_element))
    (set `Bubble.Speed` (`self.NewSpeed`) _bubbleactor)
    (set `Bubble.bShouldCoolide` true _bubbleactor)
    (set `Bubble.bShouldMove` true _bubbleactor)
    (`self.SetLifeSpan` _returnvalue_2 (`self.LifeSpan`))))

(fn `GetBubbleActor`
  (returns (BubbleActor :type "Bubble Object Reference"))
  (return self))

(fn `UserConstructionScript`
  (`parent.UserConstructionScript`))