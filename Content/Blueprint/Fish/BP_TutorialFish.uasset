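; Tutorial fish that, when a bubble overlaps its sphere, plays a sound, grants a random bubble upgrade and starts a narrative dialogue once.
; Upgrades raise lifetime, speed or max size, or lower minimum charge time on every Bubble_ShooterInterface actor.
; The pick re-rolls at each nested branch, so odds are uneven and sometimes no upgrade applies.
; Only the dialogue is gated by DoOnce; sound and upgrade repeat on each bubble hit.
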(event `self.SphereCollider.OnComponentBeginOverlap`
  (params (OverlappedComponent :type "PrimitiveComponent Object Reference") (OtherActor :type "Actor Object Reference") (OtherComp :type "PrimitiveComponent Object Reference") (OtherBodyIndex :type Integer) (bFromSweep :type Boolean) (SweepResult :type "HitResult Structure (by ref)"))
  (bind _bubbleactor (message `/Game/Blueprint/Weapon/Bubble_Interface.GetBubbleActor` OtherActor))
  (if (== _bubbleactor OtherActor)
    (`GameplayStatics.PlaySound2D` "/Game/SFX/MS_GoldFish.MS_GoldFish" 1.0 1.0 0.0 null null)
    (`self.GetRandomUpgrade`)
    (`/Engine/EditorBlueprintResources/StandardMacros.DoOnce` false
      (:`Completed`
        (bind _returnvalue (`GameplayStatics.GetActorOfClass` "/Game/Blueprint/NarrativeManager/BP_NarrativeManager.BP_NarrativeManager_C"))
        (`NarrativeManager.StartDialogue` _returnvalue "/Game/Data/Dialogue12.Dialogue12")))))

(fn `GetRandomUpgrade`
  (bind _returnvalue (`KismetMathLibrary.RandomIntegerInRange` 1 4))
  (`KismetSystemLibrary.PrintString` "choosing random upgrade")
  (if (== _returnvalue 1)
    (`self.LifeTimeUpgrade`)
    (elif (== _returnvalue 2)
      (`self.SpeedUpgrade`)
      (elif (== _returnvalue 3)
        (`self.SizeUpgrade`)
        (elif (== _returnvalue 4)
          (`self.MinChargeTimeUpgrade`))))))

(fn `LifeTimeUpgrade`
  (`KismetSystemLibrary.PrintString` "LifeTimeUpgrade")
  (bind _outactors (`GameplayStatics.GetAllActorsWithInterface` "/Game/Blueprint/Weapon/Bubble_ShooterInterface.Bubble_ShooterInterface_C"))
  (for _array_element _outactors
    (bind _lifetime (message `/Game/Blueprint/Weapon/Bubble_ShooterInterface.GetBubbleLifeTime` _array_element))
    (bind _result (`/Engine/EditorBlueprintResources/StandardMacros.IncrementFloat` _lifetime)
      (:`  `
        (message `/Game/Blueprint/Weapon/Bubble_ShooterInterface.SetBubbleLifeTime` _array_element _result)
        (`KismetSystemLibrary.PrintString` "BubbleUpgraded!")))))

(fn `MinChargeTimeUpgrade`
  (`KismetSystemLibrary.PrintString` "MinChargeTimeUpgrade")
  (bind _outactors (`GameplayStatics.GetAllActorsWithInterface` "/Game/Blueprint/Weapon/Bubble_ShooterInterface.Bubble_ShooterInterface_C"))
  (for _array_element _outactors
    (bind _minchargetime (message `/Game/Blueprint/Weapon/Bubble_ShooterInterface.GetBubbleMinChargeTime` _array_element))
    (message `/Game/Blueprint/Weapon/Bubble_ShooterInterface.SetBubbleMinChargeTime` _array_element (- _minchargetime 0.005))
    (`KismetSystemLibrary.PrintString` "BubbleUpgraded!")))

(fn `SizeUpgrade`
  (`KismetSystemLibrary.PrintString` "SizeUpgrade")
  (bind _outactors (`GameplayStatics.GetAllActorsWithInterface` "/Game/Blueprint/Weapon/Bubble_ShooterInterface.Bubble_ShooterInterface_C"))
  (for _array_element _outactors
    (bind _bubblemaxsize (message `/Game/Blueprint/Weapon/Bubble_ShooterInterface.GetBubbleMaxSize` _array_element))
    (message `/Game/Blueprint/Weapon/Bubble_ShooterInterface.SetBubbleMaxSize` _array_element (+ _bubblemaxsize 0.05))
    (`KismetSystemLibrary.PrintString` "BubbleUpgraded!")))

(fn `SpeedUpgrade`
  (`KismetSystemLibrary.PrintString` "SpeedUpgrade")
  (bind _outactors (`GameplayStatics.GetAllActorsWithInterface` "/Game/Blueprint/Weapon/Bubble_ShooterInterface.Bubble_ShooterInterface_C"))
  (for _array_element _outactors
    (bind _bubblespeed (message `/Game/Blueprint/Weapon/Bubble_ShooterInterface.GetBubbleSpeed` _array_element))
    (message `/Game/Blueprint/Weapon/Bubble_ShooterInterface.SetBubbleSpeed` _array_element (+ _bubblespeed 150.0))
    (`KismetSystemLibrary.PrintString` "BubbleUpgraded!")))

(fn `UserConstructionScript`)