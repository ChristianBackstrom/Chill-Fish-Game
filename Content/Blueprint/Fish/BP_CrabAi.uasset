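; BP_CrabAi is a crab Blueprint that wanders randomly through the level.
; On BeginPlay it waits a random delay between its min and max settings, then moves via AI MoveTo to a random point in a box around its current nav location, sized by MaxMoveDistance.
; Success restarts the wait and move cycle, while failure retries with a new point after a brief delay.
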(event `self.ReceiveBeginPlay`
  (bind _returnvalue (* (`self.MaxMoveDistance`) 100.0))
  ;[1 1 1] Take current post + random point in box as destination. Try to move to point, if works wait then do it again. if not try again
  (`KismetSystemLibrary.Delay` (`KismetMathLibrary.RandomFloatInRange` (`self.MinDelayBeforeMove`) (`self.MaxDelayBeforeMove`)) :!label _label)
  (`|AIMoveTo` self (+ (`self.GetNavAgentLocation`) (`KismetMathLibrary.RandomPointInBoundingBox` (0.0 0.0 0.0) (`KismetMathLibrary.MakeVector` _returnvalue _returnvalue _returnvalue))) null 1.0 :!label _label_2
    (:`OnSuccess`
      (goto _label))
    (:`OnFail`
      (`KismetSystemLibrary.Delay` 0.1)
      (goto _label_2))))

(fn `UserConstructionScript`)