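; Upgrade fish that, when caught, grants one random bubble stat upgrade: longer lifetime, higher speed, larger max size or shorter minimum charge time.
; The chosen upgrade adjusts that stat on every actor implementing Bubble_ShooterInterface through interface getters and setters.
; It then shows a matching icon widget and starts a fast looping timer, with IconFloatUp raising the icon and turning it toward the player for one second.
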(event `self.FishCaught`
  (`self.GetRandomUpgrade`))

(fn `GetRandomUpgrade`
  (locals (Images :type "Array of Texture2D Object Reference") (UpgradeIndex :type Integer :default 0))
  (bind _output_get (set `local.UpgradeIndex` (`KismetMathLibrary.RandomIntegerInRange` 0 3)))
  (switch `int` _output_get
    (:`0`
      (`self.LifeTimeUpgrade`))
    (:`1`
      (`self.SpeedUpgrade`))
    (:`2`
      (`self.SizeUpgrade`))
    (:`3`
      (`self.MinChargeTimeUpgrade`)))
  (bind _returnvalue (`|CreateWidget` "/Game/UI/Hints/WBP_SmallUpgrade.WBP_SmallUpgrade_C"))
  (`/Game/UI/Hints/WBP_SmallUpgrade.SetImage` _returnvalue (`|GetArrayItem` (`local.Images`) (`local.UpgradeIndex`)))
  (`WidgetComponent.SetWidget` (`self.Icon`) _returnvalue)
  (set `self.Time` (`GameplayStatics.GetTimeSeconds`))
  (`KismetSystemLibrary.K2_SetTimerDelegate` (`|CreateDelegate` :!event `IconFloatUp`) 0.001 true))

(fn `IconFloatUp`
  (locals (RelativeTime :type "Float (double-precision)"))
  (bind _output_get (set `local.RelativeTime` (- (`GameplayStatics.GetTimeSeconds`) (`self.Time`))))
  (if (>= _output_get 1.0)
    (`KismetSystemLibrary.K2_ClearTimer` null "IconFloatUp")
    (else
      (`SceneComponent.K2_AddWorldOffset` (`self.Icon`) (0.0 0.0 0.2) false false)
      (`SceneComponent.K2_SetWorldRotation` (`self.Icon`) (`KismetMathLibrary.Conv_VectorToRotator` (- (`self.K2_GetActorLocation` (`GameplayStatics.GetPlayerPawn` 0)) (`SceneComponent.K2_GetComponentLocation` (`self.Icon`)))) false false))))

(fn `LifeTimeUpgrade`
  (`KismetSystemLibrary.PrintString` "LifeTimeUpgrade")
  (bind _outactors (`GameplayStatics.GetAllActorsWithInterface` "/Game/Blueprint/Weapon/Bubble_ShooterInterface.Bubble_ShooterInterface_C"))
  (for _array_element _outactors
    (bind _lifetime (message `/Game/Blueprint/Weapon/Bubble_ShooterInterface.GetBubbleLifeTime` _array_element))
    (message `/Game/Blueprint/Weapon/Bubble_ShooterInterface.SetBubbleLifeTime` _array_element (+ _lifetime (`self.LifeUpgarde`)))
    (`KismetSystemLibrary.PrintString` "BubbleUpgraded!")))

(fn `MinChargeTimeUpgrade`
  (`KismetSystemLibrary.PrintString` "MinChargeTimeUpgrade")
  (bind _outactors (`GameplayStatics.GetAllActorsWithInterface` "/Game/Blueprint/Weapon/Bubble_ShooterInterface.Bubble_ShooterInterface_C"))
  (for _array_element _outactors
    (bind _minchargetime (message `/Game/Blueprint/Weapon/Bubble_ShooterInterface.GetBubbleMinChargeTime` _array_element))
    (message `/Game/Blueprint/Weapon/Bubble_ShooterInterface.SetBubbleMinChargeTime` _array_element (- _minchargetime (`self.MinChargeTimeUpgarde`)))
    (`KismetSystemLibrary.PrintString` "BubbleUpgraded!")))

(fn `SizeUpgrade`
  (`KismetSystemLibrary.PrintString` "SizeUpgrade")
  (bind _outactors (`GameplayStatics.GetAllActorsWithInterface` "/Game/Blueprint/Weapon/Bubble_ShooterInterface.Bubble_ShooterInterface_C"))
  (for _array_element _outactors
    (bind _bubblemaxsize (message `/Game/Blueprint/Weapon/Bubble_ShooterInterface.GetBubbleMaxSize` _array_element))
    (message `/Game/Blueprint/Weapon/Bubble_ShooterInterface.SetBubbleMaxSize` _array_element (+ _bubblemaxsize (`self.SizeUpgarde`)))
    (`KismetSystemLibrary.PrintString` "BubbleUpgraded!")))

(fn `SpeedUpgrade`
  (`KismetSystemLibrary.PrintString` "SpeedUpgrade")
  (bind _outactors (`GameplayStatics.GetAllActorsWithInterface` "/Game/Blueprint/Weapon/Bubble_ShooterInterface.Bubble_ShooterInterface_C"))
  (for _array_element _outactors
    (bind _bubblespeed (message `/Game/Blueprint/Weapon/Bubble_ShooterInterface.GetBubbleSpeed` _array_element))
    (message `/Game/Blueprint/Weapon/Bubble_ShooterInterface.SetBubbleSpeed` _array_element (+ _bubblespeed (`self.SpeedUpgarde`)))
    (`KismetSystemLibrary.PrintString` "BubbleUpgraded!")))

(fn `UserConstructionScript`)