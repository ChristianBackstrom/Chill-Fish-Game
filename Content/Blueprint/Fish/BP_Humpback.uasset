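; BP_Humpback is the humpback fish actor in what appears to be a fishing game, with a widget that shows its name.
; On BeginPlay it binds to the time slow event exposed through the game mode and applies the received value as its own CustomTimeDilation.
; It also passes its Fish type enum, converted to a string, to the WBP_FishNames widget as the displayed name.
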(event `self.ReceiveBeginPlay`
  (`|ExecutionSequence`
    (:`then_0`
      (bind _gamemode (message `/Game/Blueprint/BP_GameMode_Interface.GetFishingGameMode` (`GameplayStatics.GetGameMode`)))
      (add `/Game/Blueprint/BP_FishingGamemode.TimeSlowEvent` _gamemode (delegate `CustomEvent`)))
    (:`then_1`
      (bind _aswbp_fish_names (cast `/Game/UI/WBP_FishNames` (`WidgetComponent.GetUserWidgetObject` (`self.Widget`))))
      (`/Game/UI/WBP_FishNames.SetFishName` _aswbp_fish_names (`|GetEnumeratorNameAsString` (`.Type` (break `Fish` (`self.Fish`))))))))

(event `CustomEvent`
  (params (timedilation :type "Float (double-precision)"))
  (set `self.CustomTimeDilation` timedilation))

(fn `UserConstructionScript`)